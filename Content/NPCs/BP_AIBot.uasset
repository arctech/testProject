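; BP_AIBot is an AI bot NPC that uses PawnSensing to react to seeing or hearing a ThirdPersonCharacter.
; On sight, it draws a debug line from its facing arrow to the character and calls SimpleMoveToLocation toward that character's AITargetLocation.
; On hearing, it only visualizes the noise instigator with a debug line and sphere, without moving.
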(event OnSeePawn(PawnSensing)
  (params (Pawn :type Pawn%20Object%20Reference))
  (bind _asthird_person_character (Utilities|Casting|CastToThirdPersonCharacter Pawn))
  (Rendering|Debug|DrawDebugLine (Transformation|GetWorldLocation (Variables|Default|GetFacingArrow)) (Transformation|GetWorldLocation (Variables|/Script/Engine.Character|GetCapsuleComponent _asthird_person_character)) "(R=0.069136,G=0.000000,B=1.000000,A=1.000000)" 1.0 0.0)
  (AI|Navigation|SimpleMovetoLocation 0 (Variables|/Game/Player_ThirdPersonBP/Blueprints/ThirdPersonCharacter.ThirdPersonCharacter_C|GetAI_TargetLocation _asthird_person_character)))

(event OnHearNoise(PawnSensing)
  (params (Instigator :type Pawn%20Object%20Reference) (Location :type Vector%20%28by%20ref%29 :default "0, 0, 0") (Volume :type Float%20%28single-precision%29))
  (bind _rootcomponent (Variables|/Script/Engine.Actor|GetRootComponent Instigator))
  (bind _returnvalue (Transformation|GetWorldLocation _rootcomponent))
  (Utilities|Casting|CastToThirdPersonCharacter Instigator)
  (Rendering|Debug|DrawDebugLine (Transformation|GetWorldLocation (Variables|Default|GetFacingArrow)) _returnvalue "(R=0.000000,G=0.281250,B=0.154240,A=1.000000)" 1.0 0.0)
  (Rendering|Debug|DrawDebugSphere _returnvalue 4e+01 12 "(R=1.000000,G=1.000000,B=1.000000,A=1.000000)" 1.0))

(event EventBeginPlay)

(event Collision|EventActorBeginOverlap
  (params (OtherActor :type Actor%20Object%20Reference)))

(event EventTick
  (params (DeltaSeconds :type Float%20%28single-precision%29)))

(fn ConstructionScript)