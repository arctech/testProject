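; Ocean water body Blueprint that notifies ThirdPersonCharacter actors when they enter or leave its volume.
; Begin and end overlap cast the other actor and call its water volume enter or exit handler.
; The height argument comes from the spline component's world Z, stringified behind a "Water Height" label and parsed back to float, so the text prefix likely loses the value.
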(event EventBeginPlay)

(event Collision|EventActorBeginOverlap
  (params (OtherActor :type Actor%20Object%20Reference))
  (bind _asthird_person_character (Utilities|Casting|CastToThirdPersonCharacter OtherActor))
  (Default|HandleWaterVolumeEnterEvt _asthird_person_character (Math|Conversions|ToFloat(Integer) (Utilities|String|Append "Water Height" (Utilities|String|ToString(Float) (.z (Transformation|GetWorldLocation (Variables|Default|GetSplineComp))))))))

(event EventTick
  (params (DeltaSeconds :type Float%20%28single-precision%29)))

(event Collision|EventActorEndOverlap
  (params (OtherActor :type Actor%20Object%20Reference))
  (bind _asthird_person_character (Utilities|Casting|CastToThirdPersonCharacter OtherActor))
  (Default|HandleWaterVolumeExitEvt _asthird_person_character (Math|Conversions|ToFloat(Integer) (Utilities|String|Append "Water Height" (Utilities|String|ToString(Float) (.z (Transformation|GetWorldLocation (Variables|Default|GetSplineComp))))))))

(fn ConstructionScript)