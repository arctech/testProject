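; BP_Hoverboard is a hoverboard Blueprint that pushes its Cube off surfaces with trace-driven force.
; Each Tick, a debug-drawn downward line trace from Sphere1 applies force along the hit normal, fading linearly from HoverForce to zero over LineTraceDepth.
; Hits also set linear and angular damping on the Cube.
; Sphere traces from the other four sphere components run without an end point, and their results are unused.
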(event EventBeginPlay)

(event Collision|EventActorBeginOverlap
  (params (OtherActor :type Actor%20Object%20Reference)))

(event EventTick
  (params (DeltaSeconds :type Float%20%28single-precision%29))
  (bind _sphere1 (Variables|Default|GetSphere1))
  (bind _linetracedepth (Variables|Default|GetLineTraceDepth))
  (bind _cube (Variables|Default|GetCube))
  (bind _returnvalue (Transformation|GetWorldLocation _sphere1))
  (Utilities|FlowControl|Sequence
    (:then_0
      (bind (_outhit _returnvalue_2) (Collision|LineTraceByChannel _returnvalue (- _returnvalue (Math|Vector|MakeVector 0.0 0.0 _linetracedepth)) "TraceTypeQuery1" false 0 "ForOneFrame"))
      (if _returnvalue_2
        (Physics|AddForce _cube (* (.ImpactNormal (Collision|BreakHitResult _outhit)) (Math|Float|Lerp (Variables|Default|GetHoverForce) 0.0 (/ (Math|Vector|VectorLength (- (.Location (Collision|BreakHitResult _outhit)) _returnvalue)) _linetracedepth))) "None" false)
        (Class|PrimitiveComponent|SetLinearDamping _cube (Variables|Default|GetLinearDamping))
        (Class|PrimitiveComponent|SetAngularDamping _cube (Variables|Default|GetAngularDamping))))
    (:then_1
      (Collision|SphereTraceByChannel (Transformation|GetWorldLocation (Variables|Default|GetSphere2)) "0, 0, 0" 0.0 "TraceTypeQuery1" false 0 "None"))
    (:then_2
      (Collision|SphereTraceByChannel (Transformation|GetWorldLocation (Variables|Default|GetSphere3)) "0, 0, 0" 0.0 "TraceTypeQuery1" false 0 "None"))
    (:then_3
      (Collision|SphereTraceByChannel (Transformation|GetWorldLocation (Variables|Default|GetSphere)) "0, 0, 0" 0.0 "TraceTypeQuery1" false 0 "None"))
    (:then_4
      (Collision|SphereTraceByChannel (Transformation|GetWorldLocation (Variables|Default|GetSphere4)) "0, 0, 0" 0.0 "TraceTypeQuery1" false 0 "None"))))

(fn ConstructionScript)