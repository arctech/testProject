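; BP_Test is a test actor that switches a point light on while the player's third-person character is inside a sphere trigger.
; The construction script hides the light.
; Sphere begin and end overlap events filter for ThirdPersonCharacter, then show or hide the light and print an inside or outside debug message.
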(event OnComponentBeginOverlap(SphereTrigger)
  (params (OverlappedComponent :type Primitive%20Component%20Object%20Reference) (OtherActor :type Actor%20Object%20Reference) (OtherComp :type Primitive%20Component%20Object%20Reference) (OtherBodyIndex :type Integer) (bFromSweep :type Boolean) (SweepResult :type Hit%20Result%20Structure%20%28by%20ref%29))
  (bind _asthird_person_character (Utilities|Casting|CastToThirdPersonCharacter OtherActor))
  (Development|PrintString "Inside" true true "(R=0.000000,G=0.660000,B=1.000000,A=1.000000)" 2.0)
  (Rendering|SetVisibility (Variables|Default|GetPointLight) true false))

(event OnComponentEndOverlap(SphereTrigger)
  (params (OverlappedComponent :type Primitive%20Component%20Object%20Reference) (OtherActor :type Actor%20Object%20Reference) (OtherComp :type Primitive%20Component%20Object%20Reference) (OtherBodyIndex :type Integer))
  (Utilities|Casting|CastToThirdPersonCharacter OtherActor)
  (Development|PrintString "outside" true true "(R=0.000000,G=0.660000,B=1.000000,A=1.000000)" 2.0)
  (Rendering|SetVisibility (Variables|Default|GetPointLight) false false))

(event EventBeginPlay)

(event Collision|EventActorBeginOverlap
  (params (OtherActor :type Actor%20Object%20Reference)))

(event EventTick
  (params (DeltaSeconds :type Float%20%28single-precision%29)))

(fn ConstructionScript
  (Rendering|SetVisibility (Variables|Default|GetPointLight) false false))