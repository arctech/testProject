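; BP_Projectile is a projectile actor that emits a noise event at its impact location, with debug feedback.
; Sphere collision hits call HandleProjectileCollision, which prints a message, draws a debug sphere and calls MakeNoise with a Loudness variable.
; When projectile movement stops, it prints and draws a second debug sphere at the impact point.
; DestroyActor is unconnected, so this graph never destroys the projectile; the bounce event is empty.
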(event OnProjectileStop(ProjectileMovement)
  (params (ImpactResult :type Hit%20Result%20Structure%20%28by%20ref%29))
  (Rendering|Debug|DrawDebugSphere (.ImpactPoint (Collision|BreakHitResult ImpactResult)) 1e+02 12 "(R=0.028321,G=0.000000,B=1.000000,A=1.000000)" 2.0)
  (Development|PrintString "Projectile End!!"))

(event OnProjectileBounce(ProjectileMovement)
  (params (ImpactResult :type Hit%20Result%20Structure%20%28by%20ref%29) (ImpactVelocity :type Vector%20%28by%20ref%29 :default "0, 0, 0")))

(event OnComponentHit(SphereCollision)
  (params (HitComponent :type Primitive%20Component%20Object%20Reference) (OtherActor :type Actor%20Object%20Reference) (OtherComp :type Primitive%20Component%20Object%20Reference) (NormalImpulse :type Vector :default "0, 0, 0") (Hit :type Hit%20Result%20Structure%20%28by%20ref%29))
  (Utilities|HandleProjectileCollision Hit))

(event EventBeginPlay)

(event Collision|EventActorBeginOverlap
  (params (OtherActor :type Actor%20Object%20Reference)))

(event EventTick
  (params (DeltaSeconds :type Float%20%28single-precision%29)))

(fn ConstructionScript)