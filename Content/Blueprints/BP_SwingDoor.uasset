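; Double-wing swing door that opens for the ThirdPersonCharacter and closes again when it leaves.
; Begin overlap on SphereTrigger plays two timelines that yaw the right and left wing arrow components.
; End overlap on a separate SphereTrigger2 reverses both timelines and prints a closing message.
; An IsDoorOpen flag gates both events so the door only opens when closed and closes when open.
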(event OnComponentEndOverlap(SphereTrigger2)
  (params (OverlappedComponent :type Primitive%20Component%20Object%20Reference) (OtherActor :type Actor%20Object%20Reference) (OtherComp :type Primitive%20Component%20Object%20Reference) (OtherBodyIndex :type Integer))
  (Utilities|Casting|CastToThirdPersonCharacter OtherActor)
  (if (Variables|Default|GetisDoorOpen?)
    (Utilities|FlowControl|Sequence
      (:then_0
        ;[1 1 1] Open Door
        (bind _rotationangle (Timeline|Timeline_0 Reverse)
          (:Update
            (Transformation|SetRelativeRotation (Variables|Default|GetRightWingArrow) (Math|Rotator|MakeRotator 0.0 0.0 _rotationangle) false false))))
      (:then_1
        (bind _rotationangle_2 (Timeline|Timeline_1 Reverse)
          (:Update
            (Transformation|SetRelativeRotation (Variables|Default|GetLeftWingArrow) (Math|Rotator|MakeRotator 0.0 0.0 _rotationangle_2) false false))))
      (:then_2
        (Variables|Default|SetisDoorOpen? false)
        (Development|PrintString "Door closing")))))

(event OnComponentBeginOverlap(SphereTrigger)
  (params (OverlappedComponent :type Primitive%20Component%20Object%20Reference) (OtherActor :type Actor%20Object%20Reference) (OtherComp :type Primitive%20Component%20Object%20Reference) (OtherBodyIndex :type Integer) (bFromSweep :type Boolean) (SweepResult :type Hit%20Result%20Structure%20%28by%20ref%29))
  (Utilities|Casting|CastToThirdPersonCharacter OtherActor)
  (if (not (Variables|Default|GetisDoorOpen?))
    ;[1 1 1] Open Door
    (Utilities|FlowControl|Sequence
      (:then_0
        (bind _rotationangle (Timeline|Timeline_0 Play)
          (:Update
            (Transformation|SetRelativeRotation (Variables|Default|GetRightWingArrow) (Math|Rotator|MakeRotator 0.0 0.0 _rotationangle) false false))))
      (:then_1
        (bind _rotationangle_2 (Timeline|Timeline_1 Play)
          (:Update
            (Transformation|SetRelativeRotation (Variables|Default|GetLeftWingArrow) (Math|Rotator|MakeRotator 0.0 0.0 _rotationangle_2) false false))))
      (:then_2
        (Variables|Default|SetisDoorOpen? true)))))

(event EventBeginPlay)

(event Collision|EventActorBeginOverlap
  (params (OtherActor :type Actor%20Object%20Reference)))

(fn ConstructionScript)