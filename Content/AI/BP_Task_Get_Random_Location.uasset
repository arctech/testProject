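; Behavior tree task that picks a random reachable point within a radius around the controlled pawn's location.
; It writes the point to a blackboard key, prints debug text of point, radius and pawn location, then finishes with the query's success flag.
; The pure navigation query re-evaluates for each step, so the stored point, printed point and result come from separate random samples.
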(event EventReceiveExecuteAI
  (params (OwnerController :type AI%20Controller%20Object%20Reference) (ControlledPawn :type Pawn%20Object%20Reference))
  (bind _returnvalue (Transformation|GetActorLocation ControlledPawn))
  (bind _radius (Variables|Default|GetRadius))
  (bind (_randomlocation _returnvalue_2) (AI|Navigation|GetRandomReachablePointinRadius _returnvalue _radius 0 0))
  (AI|BehaviorTree|SetBlackboardValueasVector (Variables|Default|GetBlackboardKey) _randomlocation)
  (Development|PrintString (Utilities|String|Append (Utilities|String|ToString(Vector) _randomlocation) (Utilities|String|Append (Utilities|String|ToString(Float) _radius) (Utilities|String|ToString(Vector) _returnvalue))))
  (AI|BehaviorTree|FinishExecute _returnvalue_2))