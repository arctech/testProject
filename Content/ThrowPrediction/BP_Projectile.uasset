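; A thrown projectile, in the ThrowPrediction folder, that emits a noise where it hits.
; On BeginPlay it copies its Velocity variable into ProjectileMovement, and the construction script scales its static mesh down to a very small size.
; HandleProjectileCollision prints a debug message, draws a debug sphere and calls MakeNoise at the hit location.
; Its DestroyActor node is unconnected, so the handler leaves the projectile alive.
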(event EventBeginPlay
  (Variables|/Script/Engine.MovementComponent|SetVelocity (Variables|Default|GetProjectileMovement) (Variables|Default|GetVelocity)))

(event Collision|EventActorBeginOverlap
  (params (OtherActor :type Actor%20Object%20Reference)))

(fn ConstructionScript
  (Transformation|SetWorldScale3D (Variables|Default|GetStaticMesh) "0.030000,0.030000,0.030000"))